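; BP_AI1 is a simple chaser enemy that triggers the Lose screen when it hits the first-person character.
; An overlap on its Collision component stores whichever actor entered, without filtering, and clears it when an overlap ends.
; While set, Tick prints the target's name, turns to face it and applies a forward impulse to the Sphere.
; Hitting the player destroys the enemy, adds the Lose widget and shows the cursor.
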(event OnComponentBeginOverlap(Collision)
  (params (OverlappedComponent :type Primitive%20Component%20Object%20Reference) (OtherActor :type Actor%20Object%20Reference) (OtherComp :type Primitive%20Component%20Object%20Reference) (OtherBodyIndex :type Integer) (bFromSweep :type Boolean) (SweepResult :type Hit%20Result%20Structure%20%28by%20ref%29))
  (Variables|Default|SetbCollision true)
  (Variables|Default|SetHitActor OtherActor))

(event OnComponentEndOverlap(Collision)
  (params (OverlappedComponent :type Primitive%20Component%20Object%20Reference) (OtherActor :type Actor%20Object%20Reference) (OtherComp :type Primitive%20Component%20Object%20Reference) (OtherBodyIndex :type Integer))
  (Variables|Default|SetbCollision false)
  (Variables|Default|SetHitActor 0))

(event Custom|CustomEvent_0
  (bind _self self)
  (bind _hitactor (Variables|Default|GetHitActor))
  (Development|PrintString (Utilities|GetDisplayName _hitactor) true true "(R=0.000000,G=0.660000,B=1.000000,A=1.000000)" 0.0)
  (Transformation|SetActorRotation _self (Math|Rotator|FindLookatRotation (Transformation|GetActorLocation _self) (Transformation|GetActorLocation _hitactor)))
  (Physics|AddImpulse (Variables|Default|GetSphere) (* (Math|Vector|GetForwardVector (Variables|Default|GetArrow)) 750) "None" false))

(event EventBeginPlay)

(event Collision|EventActorBeginOverlap
  (params (OtherActor :type Actor%20Object%20Reference)))

(event EventTick
  (params (DeltaSeconds :type Float%20%28single-precision%29))
  (if (Variables|Default|GetbCollision)
    (CallFunction|CustomEvent0)))

(event Collision|EventHit
  (params (MyComp :type Primitive%20Component%20Object%20Reference) (Other :type Actor%20Object%20Reference) (OtherComp :type Primitive%20Component%20Object%20Reference) (bSelfMoved :type Boolean) (HitLocation :type Vector :default "0, 0, 0") (HitNormal :type Vector :default "0, 0, 0") (NormalImpulse :type Vector :default "0, 0, 0") (Hit :type Hit%20Result%20Structure%20%28by%20ref%29))
  (bind _returnvalue (Game|GetPlayerController 0))
  (Utilities|Casting|CastToFirstPersonCharacter Other)
  (Actor|DestroyActor)
  (bind _returnvalue_2 (UserInterface|CreateWidget "/Game/Ashleys_stuff/lose.lose_C"))
  (UserInterface|Viewport|AddtoViewport _returnvalue_2 0)
  (Variables|/Script/Engine.PlayerController|SetbShowMouseCursor _returnvalue true)
  (Input|SetIgnoreMoveInput _returnvalue false))

(fn ConstructionScript)